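; BP_Table is a game board actor that spawns and manages a grid of ClickArea cells.
; On BeginPlay it spawns a ClickArea at each component tagged SpawnPoint and stores them in SpawnedClickArea.
; Each cell's Row and Col come from single characters at fixed positions in the spawn point component's name, so the layout depends on that naming.
; LockClickArea and ResetTable loop over the stored cells to lock or reset the whole board.
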(event `self.ReceiveBeginPlay`
  ;[1 1 1] 棋盘初始化，在SpawnPoint生成ClickArea点击区域，并根据名字设定其Row和Col属性，将生成的所有ClickArea存入数组
  (for (_array_element _array_index) (`self.GetComponentsByTag` "/Script/Engine.ActorComponent" "SpawnPoint")
    (bind _returnvalue (`|SpawnActorFromClass` "/Game/ClickArea.ClickArea_C" (`KismetMathLibrary.MakeTransform` (`SceneComponent.K2_GetComponentLocation` (cast `SceneComponent` _array_element :!pure true))) "Undefined" "OverrideRootScale" null 0 0 null))
    (bind _returnvalue_2 (`KismetStringLibrary.GetCharacterArrayFromString` (`KismetSystemLibrary.GetObjectName` _array_element)))
    (set `/Game/ClickArea.Row` (`KismetStringLibrary.Conv_StringToInt` (`|GetArrayItem` _returnvalue_2 10)) _returnvalue)
    (set `/Game/ClickArea.Col` (`KismetStringLibrary.Conv_StringToInt` (`|GetArrayItem` _returnvalue_2 11)) _returnvalue)
    (`KismetArrayLibrary.Array_Set` (`self.SpawnedClickArea`) _array_index _returnvalue true)))

(event `LockClickArea`
  ;[1 1 1] 锁住所有ClickArea
  (for _array_element (`self.SpawnedClickArea`)
    (set `/Game/ClickArea.isLocked` true _array_element)))

(event `ResetTable`
  ;[1 1 1] Reset棋盘
  (for _array_element (`self.SpawnedClickArea`)
    (`/Game/ClickArea.ResetClickArea` _array_element)))

(fn `UserConstructionScript`)